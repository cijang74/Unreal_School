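; P-38 plane Blueprint that provides movement, counter-rotating propeller spin and rocket firing.
; The construction script gathers three fire transform components into an array, and the Fire! event spawns a BP_Rocat at each one's world transform.
; CalcurateSpeed scales MovementSpeed along local Z and PropRotSpeed into opposite roll rotations.
; TransFunction applies a given offset and two propeller rotations, though nothing in this Blueprint calls either function.
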(event Custom|Fire!
  (for _array_element (Variables|Default|GetFire_Transforms)
    (Game|SpawnActorfromClass "/Game/BP/BP_Rocat.BP_Rocat_C" (Transformation|GetWorldTransform _array_element) "Undefined" "MultiplyWithRoot" 0 0)))

(event Collision|EventActorBeginOverlap
  (params (OtherActor :type Actor%20Object%20Reference)))

(fn ConstructionScript
  ;[0.15 0.15 0.15 0.5] 에디터 내에서 사용되는 생성자 (값 세팅)
  (Variables|Default|SetFire_Transforms (Utilities|Array|MakeArray (Variables|Default|GetFire_Transform1) (Variables|Default|GetFire_Transform2) (Variables|Default|GetFire_Transform3))))

(fn CalcurateSpeed
  (params (A :type Float%20%28double-precision%29) (A2 :type Float%20%28single-precision%29))
  (bind _proprotspeed (Variables|Default|GetPropRotSpeed))
  (bind _returnvalue (* A _proprotspeed))
  (return (* A2 (Math|Vector|MakeVector 0.0 0.0 (Variables|Default|GetmovementSpeed))) (Math|Rotator|MakeRotator _returnvalue 0.0 0.0) (Math|Rotator|MakeRotator (* _returnvalue -1.0) 0.0 0.0)))

(fn TransFunction
  (params (DeltaLocation :type Vector) (DeltaRotation :type Rotator) (DeltaRotation2 :type Rotator))
  (Transformation|AddActorLocalOffset DeltaLocation false false)
  (Transformation|AddLocalRotation (Variables|Default|GetP-38_Prop_R) DeltaRotation false false)
  (Transformation|AddLocalRotation (Variables|Default|GetP-38_Prop_L) DeltaRotation2 false false))